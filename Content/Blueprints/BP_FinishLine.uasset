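; BP_FinishLine is a finish line that ends a timed VR run.
; Any overlap with its cube sets PlayerHit, writes the VRGameMode timer's minutes and seconds to the leaderboard's current-score text file, and opens VRSRMenuMap.
; Each Tick compares X positions and opens VRDQMenuMap if the VR pawn's X is below the line's without a recorded hit.
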(event `self.ReceiveTick`
  (params (DeltaSeconds :type "Float (single-precision)"))
  (bind _returnvalue_x (`KismetMathLibrary.BreakVector` (`self.K2_GetActorLocation`)))
  (bind _asvrpawn (cast `/Game/VRTemplate/Blueprints/VRPawn` (`GameplayStatics.GetPlayerCharacter` 0)))
  (bind _returnvalue_x_2 (`KismetMathLibrary.BreakVector` (`self.K2_GetActorLocation` _asvrpawn)))
  (if (> _returnvalue_x _returnvalue_x_2)
    (if (not (`self.PlayerHit?`))
      (`GameplayStatics.OpenLevel` "VRDQMenuMap"))))

(event `self.Shape_Cube.OnComponentBeginOverlap`
  (params (OverlappedComponent :type "PrimitiveComponent Object Reference") (OtherActor :type "Actor Object Reference") (OtherComp :type "PrimitiveComponent Object Reference") (OtherBodyIndex :type Integer) (bFromSweep :type Boolean) (SweepResult :type "HitResult Structure (by ref)"))
  (set `self.PlayerHit?` true)
  (bind _asvrgame_mode (cast `/Game/VRTemplate/Blueprints/VRGameMode` (`GameplayStatics.GetGameMode`)))
  (`_1_ReadWriteFile.WriteStringToFile` (`KismetStringLibrary.Concat_StrStr` (`KismetSystemLibrary.GetProjectDirectory`) "leaderboardText/currentScore.txt") (`KismetStringLibrary.BuildString_Double` (`KismetStringLibrary.BuildString_Double` "" "" (`/Game/VRTemplate/Blueprints/VRGameMode.TimerMinutes` _asvrgame_mode)) ": " (`/Game/VRTemplate/Blueprints/VRGameMode.TimerSeconds` _asvrgame_mode)))
  (`GameplayStatics.OpenLevel` "VRSRMenuMap"))

(fn `UserConstructionScript`)