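; BP_SlipperySurface is a placeable zone that makes the VR pawn slide while inside it.
; Box overlap removes the VRPawn's ground friction and lowers its walking braking deceleration, then end overlap sets both to fixed normal values rather than saved originals.
; The construction script sizes the Box and Plane in X and Y from Size with zero Z scale, and ShowPlane toggles the Plane's visibility.
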(event `self.Box.OnComponentBeginOverlap`
  (params (OverlappedComponent :type "PrimitiveComponent Object Reference") (OtherActor :type "Actor Object Reference") (OtherComp :type "PrimitiveComponent Object Reference") (OtherBodyIndex :type Integer) (bFromSweep :type Boolean) (SweepResult :type "HitResult Structure (by ref)"))
  (bind _asvrpawn (cast `/Game/VRTemplate/Blueprints/VRPawn` OtherActor))
  (bind _charactermovement (`Character.CharacterMovement` _asvrpawn))
  (set `CharacterMovementComponent.GroundFriction` 0.0 _charactermovement)
  (set `CharacterMovementComponent.BrakingDecelerationWalking` 350.0 _charactermovement))

(event `self.Box.OnComponentEndOverlap`
  (params (OverlappedComponent :type "PrimitiveComponent Object Reference") (OtherActor :type "Actor Object Reference") (OtherComp :type "PrimitiveComponent Object Reference") (OtherBodyIndex :type Integer))
  (bind _asvrpawn (cast `/Game/VRTemplate/Blueprints/VRPawn` OtherActor))
  (bind _charactermovement (`Character.CharacterMovement` _asvrpawn))
  (set `CharacterMovementComponent.GroundFriction` 8.0 _charactermovement)
  (set `CharacterMovementComponent.BrakingDecelerationWalking` 2000.0 _charactermovement))

(fn `UserConstructionScript`
  (bind _size (`self.Size`))
  (`SceneComponent.SetVisibility` (`self.Plane`) (`self.ShowPlane?`) false)
  (`SceneComponent.SetRelativeScale3D` (`self.Box`) (`KismetMathLibrary.MakeVector` _size _size))
  (`SceneComponent.SetRelativeScale3D` (`self.Plane`) (`KismetMathLibrary.MakeVector` _size _size)))