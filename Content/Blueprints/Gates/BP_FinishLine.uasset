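; Finish line gate for a VR timed run that records the player's result and loads the matching results menu level.
; Overlapping the cube saves the VRGameMode centisecond timer as the score and opens a VRSR menu.
; Tick treats the player dropping below the gate without a hit as a miss, opening a VRDQ menu and writing -1 in two-run modes.
; Project text files hold map selection, run counter and scores, choosing between one-run and two-run flow.
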(event `self.ReceiveTick`
  (params (DeltaSeconds :type "Float (single-precision)"))
  (bind (_returnvalue_x _returnvalue_y _returnvalue_z) (`KismetMathLibrary.BreakVector` (`self.K2_GetActorLocation`)))
  (bind (_returnvalue_x_2 _returnvalue_y_2 _returnvalue_z_2) (`KismetMathLibrary.BreakVector` (`self.K2_GetActorLocation` (`GameplayStatics.GetPlayerPawn` 0))))
  (bind _returnvalue (`KismetStringLibrary.Concat_StrStr` (`KismetSystemLibrary.GetProjectDirectory`) "RunCounterText/runCounter.txt"))
  (if (> _returnvalue_z _returnvalue_z_2)
    (if (not (`self.PlayerHit?`))
      (`KismetSystemLibrary.PrintString` "AHHHHHHHHHHHHHHH")
      (bind (_boutsuccess _outinfomessage _returnvalue_2) (`_1_ReadWriteFile.ReadStringFromFile` _returnvalue))
      (bind (_boutsuccess_2 _outinfomessage_2 _returnvalue_3) (`_1_ReadWriteFile.ReadStringFromFile` (`KismetStringLibrary.Concat_StrStr` (`KismetSystemLibrary.GetProjectDirectory`) "MainMenuSelectText/Map.txt")))
      (switch `int` (`KismetStringLibrary.Conv_StringToInt` _returnvalue_2)
        (:`0`
          (switch `int` (`KismetStringLibrary.Conv_StringToInt` _returnvalue_3)
            (:`0`
              (`GameplayStatics.OpenLevel` "VRDQOneRunMenuMap"))
            (:`1`
              (`_1_ReadWriteFile.WriteStringToFile` (`KismetStringLibrary.Concat_StrStr` (`KismetSystemLibrary.GetProjectDirectory`) "LeaderboardText/firstRunScore.txt") "-1")
              (`_1_ReadWriteFile.WriteStringToFile` _returnvalue "1")
              (`GameplayStatics.OpenLevel` "VRDQTwoRunsMenuMap"))
            (:`2`
              (`_1_ReadWriteFile.WriteStringToFile` (`KismetStringLibrary.Concat_StrStr` (`KismetSystemLibrary.GetProjectDirectory`) "LeaderboardText/firstRunScore.txt") "-1")
              (`_1_ReadWriteFile.WriteStringToFile` _returnvalue "1")
              (`GameplayStatics.OpenLevel` "VRDQTwoRunsMenuMap"))))
        (:`1`
          (switch `int` (`KismetStringLibrary.Conv_StringToInt` _returnvalue_3)
            (:`1`
              (`_1_ReadWriteFile.WriteStringToFile` (`KismetStringLibrary.Concat_StrStr` (`KismetSystemLibrary.GetProjectDirectory`) "LeaderboardText/currentScore.txt") "-1")
              (`_1_ReadWriteFile.WriteStringToFile` _returnvalue "2")
              (`GameplayStatics.OpenLevel` "VRDQTwoRunsMenuMap"))
            (:`2`
              (`_1_ReadWriteFile.WriteStringToFile` (`KismetStringLibrary.Concat_StrStr` (`KismetSystemLibrary.GetProjectDirectory`) "LeaderboardText/currentScore.txt") "-1")
              (`_1_ReadWriteFile.WriteStringToFile` _returnvalue "2")
              (`GameplayStatics.OpenLevel` "VRDQTwoRunsMenuMap"))))))))

(event `self.Shape_Cube.OnComponentBeginOverlap`
  (params (OverlappedComponent :type "PrimitiveComponent Object Reference") (OtherActor :type "Actor Object Reference") (OtherComp :type "PrimitiveComponent Object Reference") (OtherBodyIndex :type Integer) (bFromSweep :type Boolean) (SweepResult :type "HitResult Structure (by ref)"))
  (bind _returnvalue (`KismetStringLibrary.Concat_StrStr` (`KismetSystemLibrary.GetProjectDirectory`) "RunCounterText/runCounter.txt"))
  (`KismetSystemLibrary.PrintString` "Hit Finish Line")
  (bind _output_get (set `self.PlayerHit?` true))
  (`KismetSystemLibrary.PrintString` (`KismetStringLibrary.Conv_BoolToString` _output_get))
  (bind _asvrgame_mode (cast `/Game/VRTemplate/Blueprints/VRGameMode` (`GameplayStatics.GetGameMode`)))
  (`KismetSystemLibrary.PrintString` "Cast Pass")
  (`_1_ReadWriteFile.WriteStringToFile` (`KismetStringLibrary.Concat_StrStr` (`KismetSystemLibrary.GetProjectDirectory`) "leaderboardText/currentTime.txt") (`KismetStringLibrary.BuildString_Double` "" ": " (`/Game/VRTemplate/Blueprints/VRGameMode.TimerCentiSeconds` _asvrgame_mode)))
  (set `self.Score` (`KismetStringLibrary.BuildString_Double` "" "" (`/Game/VRTemplate/Blueprints/VRGameMode.TimerCentiSeconds` _asvrgame_mode)))
  (bind (_boutsuccess _outinfomessage _returnvalue_2) (`_1_ReadWriteFile.ReadStringFromFile` _returnvalue))
  (bind (_boutsuccess_2 _outinfomessage_2 _returnvalue_3) (`_1_ReadWriteFile.ReadStringFromFile` (`KismetStringLibrary.Concat_StrStr` (`KismetSystemLibrary.GetProjectDirectory`) "MainMenuSelectText/Map.txt")))
  (switch `int` (`KismetStringLibrary.Conv_StringToInt` _returnvalue_2)
    (:`0`
      (switch `int` (`KismetStringLibrary.Conv_StringToInt` _returnvalue_3)
        (:`0`
          (`_1_ReadWriteFile.WriteStringToFile` (`KismetStringLibrary.Concat_StrStr` (`KismetSystemLibrary.GetProjectDirectory`) "LeaderboardText/currentScore.txt") (`self.Score`))
          (`GameplayStatics.OpenLevel` "VRSROneRunMenuMap"))
        (:`1`
          (`_1_ReadWriteFile.WriteStringToFile` (`KismetStringLibrary.Concat_StrStr` (`KismetSystemLibrary.GetProjectDirectory`) "LeaderboardText/firstRunScore.txt") (`self.Score`))
          (`_1_ReadWriteFile.WriteStringToFile` _returnvalue "1")
          (`GameplayStatics.OpenLevel` "VRSRTwoRunsMenuMap"))
        (:`2`
          (`_1_ReadWriteFile.WriteStringToFile` (`KismetStringLibrary.Concat_StrStr` (`KismetSystemLibrary.GetProjectDirectory`) "LeaderboardText/firstRunScore.txt") (`self.Score`))
          (`_1_ReadWriteFile.WriteStringToFile` _returnvalue "1")
          (`GameplayStatics.OpenLevel` "VRSRTwoRunsMenuMap"))))
    (:`1`
      (switch `int` (`KismetStringLibrary.Conv_StringToInt` _returnvalue_3)
        (:`1`
          (`_1_ReadWriteFile.WriteStringToFile` (`KismetStringLibrary.Concat_StrStr` (`KismetSystemLibrary.GetProjectDirectory`) "LeaderboardText/currentScore.txt") (`self.Score`))
          (`_1_ReadWriteFile.WriteStringToFile` _returnvalue "2")
          (`GameplayStatics.OpenLevel` "VRSRTwoRunsMenuMap"))
        (:`2`
          (`_1_ReadWriteFile.WriteStringToFile` (`KismetStringLibrary.Concat_StrStr` (`KismetSystemLibrary.GetProjectDirectory`) "LeaderboardText/currentScore.txt") (`self.Score`))
          (`_1_ReadWriteFile.WriteStringToFile` _returnvalue "2")
          (`GameplayStatics.OpenLevel` "VRSRTwoRunsMenuMap"))))))

(fn `UserConstructionScript`)