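; BP_GateSpawner is an actor that spawns one scaled actor, presumably a gate going by its name, when play begins.
; It keeps its own X, Z and rotation for the spawn and picks a random Y between its PlaneLeft and PlaneRight components, inset by a margin at each side.
; The spawned class is not specified in the graph, and the construction script is empty.
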(event `self.ReceiveBeginPlay`
  (bind (_returnvalue_x _returnvalue_y _returnvalue_z) (`KismetMathLibrary.BreakVector` (`self.K2_GetActorLocation`)))
  (bind (_returnvalue_x_2 _returnvalue_y_2) (`KismetMathLibrary.BreakVector` (`SceneComponent.K2_GetComponentLocation` (`self.PlaneRight`))))
  (bind (_returnvalue_x_3 _returnvalue_y_3) (`KismetMathLibrary.BreakVector` (`SceneComponent.K2_GetComponentLocation` (`self.PlaneLeft`))))
  (bind _output_get (set `self.X` _returnvalue_x))
  (bind _output_get_2 (set `self.Z` _returnvalue_z))
  (bind _output_get_3 (set `self.Y` (`KismetMathLibrary.RandomFloatInRange` (+ _returnvalue_y_3 150.0) (- _returnvalue_y_2 150.0))))
  (`|SpawnActorFromClass` "/Game/Blueprints/BP_Gate.BP_Gate_C" (`KismetMathLibrary.MakeTransform` (`KismetMathLibrary.MakeVector` _output_get _output_get_3 _output_get_2) (`self.K2_GetActorRotation`) (1.0 3.75 2.0)) "Undefined" "OverrideRootScale" null null))

(fn `UserConstructionScript`)