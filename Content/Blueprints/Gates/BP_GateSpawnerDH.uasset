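; BP_GateSpawnerDH is a gate spawner actor whose spawn logic is currently disconnected, so it spawns nothing.
; BeginPlay only reads the actor's Z location into a string switch with no cases.
; The unconnected chain would spawn a scaled BP_Gate at the actor's X, Z and rotation, with random Y inset between PlaneLeft and PlaneRight.
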(event `self.ReceiveBeginPlay`
  (bind (_returnvalue_x _returnvalue_y _returnvalue_z) (`KismetMathLibrary.BreakVector` (`self.K2_GetActorLocation`)))
  (bind _output_get (set `self.Z` _returnvalue_z))
  (switch `string` (`KismetStringLibrary.Conv_DoubleToString` _output_get)))

(fn `UserConstructionScript`)