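; Gate spawner that places one BP_Gate at a randomly chosen spot when play begins.
; Each placed instance identifies itself by switching on its own Z location converted to a string, with four known heights supported.
; Each height picks one of three hard-coded world transforms, so moving a spawner vertically breaks the match unless its case is updated.
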(event `self.ReceiveBeginPlay`
  (bind (_returnvalue_x _returnvalue_y _returnvalue_z) (`KismetMathLibrary.BreakVector` (`self.K2_GetActorLocation`)))
  (bind _output_get (set `self.Z` _returnvalue_z))
  (switch `string` (`KismetStringLibrary.Conv_DoubleToString` _output_get)
    (:`12387.757791`
      (switch `int` (`KismetMathLibrary.RandomIntegerInRange` 0 2)
        (:`0`
          (`|SpawnActorFromClass` "/Game/Blueprints/Gates/BP_Gate.BP_Gate_C" (`KismetMathLibrary.MakeTransform` (56750.0 143040.0 12387.757812) (struct :`Pitch` 2.708546 :`Yaw` -58.94463 :`Roll` -3.73017) (1.0 3.75 2.0)) "Undefined" "OverrideRootScale" null null))
        (:`1`
          (`|SpawnActorFromClass` "/Game/Blueprints/Gates/BP_Gate.BP_Gate_C" (`KismetMathLibrary.MakeTransform` (54299.304688 143701.90625 11664.30957) (struct :`Pitch` 2.708546 :`Yaw` -58.94463 :`Roll` 5.0) (1.0 3.75 2.0)) "Undefined" "OverrideRootScale" null null))
        (:`2`
          (`|SpawnActorFromClass` "/Game/Blueprints/Gates/BP_Gate.BP_Gate_C" (`KismetMathLibrary.MakeTransform` (57277.089844 146170.46875 11832.638672) (struct :`Pitch` 12.361641 :`Yaw` -61.581749 :`Roll` -15.347105) (1.0 3.75 2.0)) "Undefined" "OverrideRootScale" null null))))
    (:`261.58685`
      (switch `int` (`KismetMathLibrary.RandomIntegerInRange` 0 2)
        (:`0`
          (`|SpawnActorFromClass` "/Game/Blueprints/Gates/BP_Gate.BP_Gate_C" (`KismetMathLibrary.MakeTransform` (34169.621094 173219.921875 1161.586792) (struct :`Pitch` 5.0 :`Yaw` -40.992828) (1.0 3.75 2.0)) "Undefined" "OverrideRootScale" null null))
        (:`1`
          (`|SpawnActorFromClass` "/Game/Blueprints/Gates/BP_Gate.BP_Gate_C" (`KismetMathLibrary.MakeTransform` (34426.539062 166982.875 2127.924072) (struct :`Yaw` -45.0 :`Roll` 10.0) (1.0 3.75 2.0)) "Undefined" "OverrideRootScale" null null))
        (:`2`
          (`|SpawnActorFromClass` "/Game/Blueprints/Gates/BP_Gate.BP_Gate_C" (`KismetMathLibrary.MakeTransform` (29117.978516 174670.59375 249.46405) (struct :`Pitch` 8.177733 :`Yaw` -35.413185 :`Roll` 4.224914) (1.0 3.75 2.0)) "Undefined" "OverrideRootScale" null null))))
    (:`-12583.64535`
      (switch `int` (`KismetMathLibrary.RandomIntegerInRange` 0 2)
        (:`0`
          (`|SpawnActorFromClass` "/Game/Blueprints/Gates/BP_Gate.BP_Gate_C" (`KismetMathLibrary.MakeTransform` (2264.778564 187995.71875 -12583.645508) (struct :`Pitch` 10.995577 :`Yaw` -37.384388 :`Roll` -2.5) (1.0 3.75 2.0)) "Undefined" "OverrideRootScale" null null))
        (:`1`
          (`|SpawnActorFromClass` "/Game/Blueprints/Gates/BP_Gate.BP_Gate_C" (`KismetMathLibrary.MakeTransform` (1613.525269 191635.328125 -13504.71875) (struct :`Pitch` 10.995577 :`Yaw` -37.384388 :`Roll` -5.0) (1.0 3.75 2.0)) "Undefined" "OverrideRootScale" null null))
        (:`2`
          (`|SpawnActorFromClass` "/Game/Blueprints/Gates/BP_Gate.BP_Gate_C" (`KismetMathLibrary.MakeTransform` (5750.445801 193418.796875 -11866.878906) (struct :`Pitch` 10.995577 :`Yaw` -37.384388 :`Roll` -10.0) (1.0 3.75 2.0)) "Undefined" "OverrideRootScale" null null))))
    (:`-21276.18317`
      (switch `int` (`KismetMathLibrary.RandomIntegerInRange` 0 2)
        (:`0`
          (`|SpawnActorFromClass` "/Game/Blueprints/Gates/BP_Gate.BP_Gate_C" (`KismetMathLibrary.MakeTransform` (-13595.65918 209418.546875 -21146.183594) (struct :`Pitch` -0.217294 :`Yaw` -51.753143 :`Roll` 1.754608) (1.0 3.75 2.0)) "Undefined" "OverrideRootScale" null null))
        (:`1`
          (`|SpawnActorFromClass` "/Game/Blueprints/Gates/BP_Gate.BP_Gate_C" (`KismetMathLibrary.MakeTransform` (-12937.698242 212753.046875 -21808.808594) (struct :`Pitch` 9.777972 :`Yaw` -51.753143) (1.0 3.75 2.0)) "Undefined" "OverrideRootScale" null null))
        (:`2`
          (`|SpawnActorFromClass` "/Game/Blueprints/Gates/BP_Gate.BP_Gate_C" (`KismetMathLibrary.MakeTransform` (-19680.611328 208937.03125 -22029.072266) (struct :`Pitch` 9.777972 :`Yaw` -51.753143 :`Roll` 1.0) (1.0 3.75 2.0)) "Undefined" "OverrideRootScale" null null))))))

(fn `UserConstructionScript`)