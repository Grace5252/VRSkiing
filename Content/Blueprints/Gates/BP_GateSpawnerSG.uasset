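; Gate spawner actor that places one BP_Gate at a randomly chosen preset spot when play begins.
; Each placed instance identifies its course position by matching its own Z location, converted to a string, against six hardcoded heights.
; Each height has three hand-tuned transforms with a shared scale, one picked at random.
; An instance whose Z does not match exactly spawns nothing.
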(event `self.ReceiveBeginPlay`
  (bind (_returnvalue_x _returnvalue_y _returnvalue_z) (`KismetMathLibrary.BreakVector` (`self.K2_GetActorLocation`)))
  (bind _output_get (set `self.Z` _returnvalue_z))
  (switch `string` (`KismetStringLibrary.Conv_DoubleToString` _output_get)
    (:`26698.304901`
      (switch `int` (`KismetMathLibrary.RandomIntegerInRange` 0 2)
        (:`0`
          (`|SpawnActorFromClass` "/Game/Blueprints/Gates/BP_Gate.BP_Gate_C" (`KismetMathLibrary.MakeTransform` (82683.3125 118113.984375 26258.304688) (struct :`Pitch` 16.917549 :`Yaw` -60.374249 :`Roll` -7.69856) (1.0 3.75 2.0)) "Undefined" "OverrideRootScale" null null))
        (:`1`
          (`|SpawnActorFromClass` "/Game/Blueprints/Gates/BP_Gate.BP_Gate_C" (`KismetMathLibrary.MakeTransform` (82553.3125 116513.0 26708.0) (struct :`Pitch` 11.25 :`Yaw` -58.94463 :`Roll` 1.51) (1.0 3.75 2.0)) "Undefined" "OverrideRootScale" null null))
        (:`2`
          (`|SpawnActorFromClass` "/Game/Blueprints/Gates/BP_Gate.BP_Gate_C" (`KismetMathLibrary.MakeTransform` (80473.3125 116733.0 26328.0) (struct :`Pitch` 11.760762 :`Yaw` -45.183224 :`Roll` 15.897431) (1.0 3.75 2.0)) "Undefined" "OverrideRootScale" null null))))
    (:`16548.120142`
      (switch `int` (`KismetMathLibrary.RandomIntegerInRange` 0 2)
        (:`0`
          (`|SpawnActorFromClass` "/Game/Blueprints/Gates/BP_Gate.BP_Gate_C" (`KismetMathLibrary.MakeTransform` (67738.859375 134386.234375 17208.121094) (struct :`Pitch` 18.660389 :`Yaw` -52.630356 :`Roll` -10.379301) (1.0 3.75 2.0)) "Undefined" "OverrideRootScale" null null))
        (:`1`
          (`|SpawnActorFromClass` "/Game/Blueprints/Gates/BP_Gate.BP_Gate_C" (`KismetMathLibrary.MakeTransform` (63268.859375 133216.234375 16908.121094) (struct :`Pitch` 15.600155 :`Yaw` -39.113033 :`Roll` 23.008516) (1.0 3.75 2.0)) "Undefined" "OverrideRootScale" null null))
        (:`2`
          (`|SpawnActorFromClass` "/Game/Blueprints/Gates/BP_Gate.BP_Gate_C" (`KismetMathLibrary.MakeTransform` (65298.859375 138416.234375 15928.120117) (struct :`Pitch` 1.62859 :`Yaw` -54.398418 :`Roll` -17.614763) (1.0 3.75 2.0)) "Undefined" "OverrideRootScale" null null))))
    (:`7884.570142`
      (switch `int` (`KismetMathLibrary.RandomIntegerInRange` 0 2)
        (:`0`
          (`|SpawnActorFromClass` "/Game/Blueprints/Gates/BP_Gate.BP_Gate_C" (`KismetMathLibrary.MakeTransform` (51038.859375 154816.234375 8138.120117) (struct :`Pitch` 12.412506 :`Yaw` -48.765705 :`Roll` -12.473426) (1.0 3.75 2.0)) "Undefined" "OverrideRootScale" null null))
        (:`1`
          (`|SpawnActorFromClass` "/Game/Blueprints/Gates/BP_Gate.BP_Gate_C" (`KismetMathLibrary.MakeTransform` (45258.246094 153649.640625 6947.504395) (struct :`Pitch` 15.600155 :`Yaw` -39.113033 :`Roll` 13.008517) (1.0 3.75 2.0)) "Undefined" "OverrideRootScale" null null))
        (:`2`
          (`|SpawnActorFromClass` "/Game/Blueprints/Gates/BP_Gate.BP_Gate_C" (`KismetMathLibrary.MakeTransform` (49658.859375 157516.234375 7158.120117) (struct :`Pitch` 11.152912 :`Yaw` -57.468658 :`Roll` -17.957773) (1.0 3.75 2.0)) "Undefined" "OverrideRootScale" null null))))
    (:`-1469.888299`
      (switch `int` (`KismetMathLibrary.RandomIntegerInRange` 0 2)
        (:`0`
          (`|SpawnActorFromClass` "/Game/Blueprints/Gates/BP_Gate.BP_Gate_C" (`KismetMathLibrary.MakeTransform` (30108.912109 175941.609375 159.647629) (struct :`Pitch` 2.4963 :`Yaw` -50.070278 :`Roll` -2.64332) (1.0 3.75 2.0)) "Undefined" "OverrideRootScale" null null))
        (:`1`
          (`|SpawnActorFromClass` "/Game/Blueprints/Gates/BP_Gate.BP_Gate_C" (`KismetMathLibrary.MakeTransform` (26533.550781 176688.59375 -686.464783) (struct :`Pitch` 15.600155 :`Yaw` -39.113033) (1.0 3.75 2.0)) "Undefined" "OverrideRootScale" null null))
        (:`2`
          (`|SpawnActorFromClass` "/Game/Blueprints/Gates/BP_Gate.BP_Gate_C" (`KismetMathLibrary.MakeTransform` (29931.380859 179463.40625 -123.778191) (struct :`Pitch` 11.152912 :`Yaw` -37.468658 :`Roll` -7.957773) (1.0 3.75 2.0)) "Undefined" "OverrideRootScale" null null))))
    (:`-16041.966368`
      (switch `int` (`KismetMathLibrary.RandomIntegerInRange` 0 2)
        (:`0`
          (`|SpawnActorFromClass` "/Game/Blueprints/Gates/BP_Gate.BP_Gate_C" (`KismetMathLibrary.MakeTransform` (674.750061 196570.859375 -14884.537109) (struct :`Pitch` 2.917268 :`Yaw` -40.067932 :`Roll` -7.0) (1.0 3.75 2.0)) "Undefined" "OverrideRootScale" null null))
        (:`1`
          (`|SpawnActorFromClass` "/Game/Blueprints/Gates/BP_Gate.BP_Gate_C" (`KismetMathLibrary.MakeTransform` (-4035.491211 196691.75 -16435.810547) (struct :`Pitch` 15.600155 :`Yaw` -39.113033 :`Roll` 2.0) (1.0 3.75 2.0)) "Undefined" "OverrideRootScale" null null))
        (:`2`
          (`|SpawnActorFromClass` "/Game/Blueprints/Gates/BP_Gate.BP_Gate_C" (`KismetMathLibrary.MakeTransform` (-53.869007 200224.359375 -15922.895508) (struct :`Pitch` 11.152912 :`Yaw` -37.468658 :`Roll` -4.0) (1.0 3.75 2.0)) "Undefined" "OverrideRootScale" null null))))
    (:`-27396.073185`
      (switch `int` (`KismetMathLibrary.RandomIntegerInRange` 0 2)
        (:`0`
          (`|SpawnActorFromClass` "/Game/Blueprints/Gates/BP_Gate.BP_Gate_C" (`KismetMathLibrary.MakeTransform` (-23341.332031 216271.375 -24688.371094) (struct :`Pitch` 10.0 :`Yaw` -40.067932 :`Roll` 3.0) (1.0 3.75 2.0)) "Undefined" "OverrideRootScale" null null))
        (:`1`
          (`|SpawnActorFromClass` "/Game/Blueprints/Gates/BP_Gate.BP_Gate_C" (`KismetMathLibrary.MakeTransform` (-27364.777344 216239.203125 -25583.96875) (struct :`Pitch` 15.600155 :`Yaw` -39.113033 :`Roll` 2.0) (1.0 3.75 2.0)) "Undefined" "OverrideRootScale" null null))
        (:`2`
          (`|SpawnActorFromClass` "/Game/Blueprints/Gates/BP_Gate.BP_Gate_C" (`KismetMathLibrary.MakeTransform` (-23278.613281 219931.28125 -25584.410156) (struct :`Pitch` 11.152912 :`Yaw` -37.468658 :`Roll` 3.0) (1.0 3.75 2.0)) "Undefined" "OverrideRootScale" null null))))))

(fn `UserConstructionScript`)