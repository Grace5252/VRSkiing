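; BP_SkiVehicle is a VR ski vehicle that is steered by tilting the headset.
; Each tick, once HMD roll passes a threshold offset from the VR origin's roll, that raw roll becomes the movement component's steering input.
; Within that same check, the handbrake engages at high forward speed and releases below it.
; Pressing W sets throttle, with no release handler, and the left movement axis event is empty.
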(event `self.ReceiveTick`
  (params (DeltaSeconds :type "Float (single-precision)"))
  (bind _vehiclemovementcomponent (`self.VehicleMovementComponent`))
  (bind _hmd (`self.HMD`))
  (bind _returnvalue_roll (`KismetMathLibrary.BreakRotator` (`SceneComponent.K2_GetComponentRotation` _hmd)))
  ;[1 1 1] VR Camera
  (if (>= (`KismetMathLibrary.Abs` (.roll (`SceneComponent.K2_GetComponentRotation` _hmd))) (`KismetMathLibrary.Abs` (+ (.roll (`SceneComponent.K2_GetComponentRotation` (`self.VROrigin`))) 5.0)))
    (`ChaosVehicleMovementComponent.SetSteeringInput` (`self.VehicleMovementComponent`) _returnvalue_roll)
    (if (>= (`ChaosVehicleMovementComponent.GetForwardSpeedMPH` _vehiclemovementcomponent) 85.0)
      (`ChaosVehicleMovementComponent.SetHandbrakeInput` _vehiclemovementcomponent true)
      (else
        (`ChaosVehicleMovementComponent.SetHandbrakeInput` _vehiclemovementcomponent false)))))

(event `InputAxis|MovementAxisLeft_Y`
  (params (AxisValue :type "Float (single-precision)")))

(event `Key|W`
  (params (Key :type "Key Structure"))
  (:`Pressed`
    (`ChaosVehicleMovementComponent.SetThrottleInput` (`self.VehicleMovementComponent`) 10.0)))

(fn `UserConstructionScript`)