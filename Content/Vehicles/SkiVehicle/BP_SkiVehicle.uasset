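; VR ski vehicle Blueprint that drives itself forward at full throttle after a start delay meant to match the VR game mode's.
; Each tick, HMD roll sets steering once it passes a threshold relative to the VR origin, and the handbrake engages as a speed cap.
; Left and right pole overlaps track ground contact and print on touch, but the two-pole check does nothing.
; Timer, friction and walk-speed braking nodes remain disconnected.
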(event `self.ReceiveTick`
  (params (DeltaSeconds :type "Float (single-precision)"))
  (bind _vehiclemovementcomponent (`self.VehicleMovementComponent`))
  (bind _hmd (`self.HMD`))
  (bind _returnvalue_roll (`KismetMathLibrary.BreakRotator` (`SceneComponent.K2_GetComponentRotation` _hmd)))
  ;[1 1 1] VR Camera
  (if (>= (`KismetMathLibrary.Abs` (.roll (`SceneComponent.K2_GetComponentRotation` _hmd))) (`KismetMathLibrary.Abs` (+ (.roll (`SceneComponent.K2_GetComponentRotation` (`self.VROrigin`))) 2.5)))
    (`ChaosVehicleMovementComponent.SetSteeringInput` (`self.VehicleMovementComponent`) (/ _returnvalue_roll 35.0)))
  (if (>= (`ChaosVehicleMovementComponent.GetForwardSpeedMPH` _vehiclemovementcomponent) 85.0)
    (`ChaosVehicleMovementComponent.SetHandbrakeInput` _vehiclemovementcomponent true)
    (else
      (`ChaosVehicleMovementComponent.SetHandbrakeInput` _vehiclemovementcomponent false))))

(event `self.ReceiveBeginPlay`
  (`KismetSystemLibrary.Delay` 3.0) ; Change VRGameMode delay to match this delay
  (`ChaosVehicleMovementComponent.SetThrottleInput` (`self.VehicleMovementComponent`) 1.0))

(event `self.LeftPole.OnComponentBeginOverlap`
  (params (OverlappedComponent :type "PrimitiveComponent Object Reference") (OtherActor :type "Actor Object Reference") (OtherComp :type "PrimitiveComponent Object Reference") (OtherBodyIndex :type Integer) (bFromSweep :type Boolean) (SweepResult :type "HitResult Structure (by ref)"))
  ;[1 1 1] Pole Logic (2 Poles, one in each hand)
  ;;[1 1 1] Initial Pole Interaction design
  (`KismetSystemLibrary.PrintString` "Left Pole Overlap")
  (bind _output_get (set `self.LeftPoleInGround` true))
  (if (and _output_get (stale `self.RightPole.OnComponentBeginOverlap` _output_get)) :!label _label
    _))

(event `self.RightPole.OnComponentBeginOverlap`
  (params (OverlappedComponent :type "PrimitiveComponent Object Reference") (OtherActor :type "Actor Object Reference") (OtherComp :type "PrimitiveComponent Object Reference") (OtherBodyIndex :type Integer) (bFromSweep :type Boolean) (SweepResult :type "HitResult Structure (by ref)"))
  ;[1 1 1] Pole Logic (2 Poles, one in each hand)
  ;;[1 1 1] Initial Pole Interaction design
  (`KismetSystemLibrary.PrintString` "Right Pole Overlap")
  (bind _output_get (set `self.RightPoleInGround` true))
  (goto _label))

(event `StillOverlap`
  ;[1 1 1] Pole Logic (2 Poles, one in each hand)
  ;;[1 1 1] Initial Pole Interaction design
  (bind _asvrpawn (cast `/Game/VRTemplate/Blueprints/VRPawn` (`GameplayStatics.GetPlayerCharacter` 0))))

(event `self.LeftPole.OnComponentEndOverlap`
  (params (OverlappedComponent :type "PrimitiveComponent Object Reference") (OtherActor :type "Actor Object Reference") (OtherComp :type "PrimitiveComponent Object Reference") (OtherBodyIndex :type Integer))
  ;[1 1 1] Pole Logic (2 Poles, one in each hand)
  ;;[1 1 1] Initial Pole Interaction design
  (bind _output_get (set `self.LeftPoleInGround` false))
  (if (and _output_get (stale `self.RightPole.OnComponentEndOverlap` _output_get)) :!label _label_2
    _))

(event `self.RightPole.OnComponentEndOverlap`
  (params (OverlappedComponent :type "PrimitiveComponent Object Reference") (OtherActor :type "Actor Object Reference") (OtherComp :type "PrimitiveComponent Object Reference") (OtherBodyIndex :type Integer))
  ;[1 1 1] Pole Logic (2 Poles, one in each hand)
  ;;[1 1 1] Initial Pole Interaction design
  (bind _output_get (set `self.RightPoleInGround` false))
  (goto _label_2))

(fn `UserConstructionScript`)